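; BP_JetpackForce is a short-lived radial force actor for the jetpack projectile that applies a physics impulse on spawn.
; On BeginPlay, UpdateFire copies radius, impulse and force strength from a data asset into its force component and fires the impulse.
; The actor destroys itself half a second later.
; ChangeAuthor resets the radius to the base value plus a passed-in bonus, without firing again.
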(event EventBeginPlay
  (CallFunction|UpdateFire)
  (Utilities|FlowControl|Delay 0.5)
  (Actor|DestroyActor))

(fn ConstructionScript)

(fn UpdateFire
  (bind _forcecomponent (Variables|Default|GetForceComponent))
  (bind _dataasset (Variables|Default|GetdataAsset))
  (Variables|/Script/Engine.RadialForceComponent|SetRadius _forcecomponent (Variables|/Game/Blueprints/Characters/JetPack/JP_DataAsset/BP_JetPackDataAsset.BP_JetPackDataAsset_C|GetBaseRadius _dataasset))
  (Variables|/Script/Engine.RadialForceComponent|SetImpulseStrength _forcecomponent (Variables|/Game/Blueprints/Characters/JetPack/JP_DataAsset/BP_JetPackDataAsset.BP_JetPackDataAsset_C|GetImpulseStrength _dataasset))
  (Variables|/Script/Engine.RadialForceComponent|SetForceStrength _forcecomponent (Variables|/Game/Blueprints/Characters/JetPack/JP_DataAsset/BP_JetPackDataAsset.BP_JetPackDataAsset_C|GetForceStrength _dataasset))
  (Class|RadialForceComponent|FireImpulse _forcecomponent))

(fn ChangeAuthor
  (params (UpAuthor :type Float%20%28double-precision%29))
  (Variables|/Script/Engine.RadialForceComponent|SetRadius (Variables|Default|GetForceComponent) (+ UpAuthor (Variables|/Game/Blueprints/Characters/JetPack/JP_DataAsset/BP_JetPackDataAsset.BP_JetPackDataAsset_C|GetBaseRadius (Variables|Default|GetdataAsset)))))