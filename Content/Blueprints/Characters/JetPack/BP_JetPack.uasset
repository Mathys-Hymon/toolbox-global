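; Jetpack Blueprint where Left Shift raises and Left Ctrl lowers a thrust/height value (NewAuthor) within fixed limits.
; While that value is above minimum, Tick drains DataAsset-defined fuel and, through a short Delay, spawns BP_JetpackProjectile at the owner's location, passing it the value.
; Fuel restores only in the empty-tank branch of that same check.
; A JetpackUI widget created on BeginPlay displays force and fuel.
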(event EventTick
  (params (DeltaSeconds :type Float%20%28single-precision%29))
  (bind _ui (Variables|Default|GetUI))
  ;[1 1 1] Change jetpack author
  (if (Variables|Default|GetDownMaxAuthor?)
    (CallFunction|DownMaxAuthor))
  (if (Variables|Default|GetUpMaxAuthor?)
    (CallFunction|UpMaxAuthor))
  ;[0 1 0.8049] Change fuel stock
  (if (> (Variables|Default|GetNewAuthor) -2e+02)
    (if (> (Variables|Default|GetActualFuel) 0.0)
      (Variables|Default|SetActualFuel (- (Variables|Default|GetActualFuel) (Variables|/Game/Blueprints/Characters/JetPack/JP_DataAsset/BP_JetPackDataAsset.BP_JetPackDataAsset_C|GetFuelConsume (Variables|Default|GetdataAsset))))
      ;[1 0.5471 0.09945] spawn jetpack force
      (Utilities|FlowControl|Delay 0.08)
      (bind _returnvalue (Game|SpawnActorfromClass "/Game/Blueprints/Characters/JetPack/JP_Projectile/BP_JetpackProjectile.BP_JetpackProjectile_C" (Math|Transform|MakeTransform (Transformation|GetActorLocation (Components|GetOwner))) "Undefined" "OverrideRootScale" 0 0))
      (Variables|/Game/Blueprints/Characters/JetPack/JP_Projectile/BP_JetpackProjectile.BP_JetpackProjectile_C|SetNewAuthor _returnvalue (Variables|Default|GetNewAuthor))
      (Default|ChangeJpForce _ui (Variables|Default|GetNewAuthor) 7e+02 -2e+02) ; Update UI
      (else
        (CallFunction|Fuel)))
    ;[0 1 0.8049] Change fuel stock
    (Default|ChangeFuel _ui (Variables|Default|GetActualFuel) (Variables|/Game/Blueprints/Characters/JetPack/JP_DataAsset/BP_JetPackDataAsset.BP_JetPackDataAsset_C|GetMaxFuel (Variables|Default|GetdataAsset))) ; Update UI
  ))

(event EventBeginPlay
  ;[1 1 1] Create jetpack UI
  (bind _returnvalue (UserInterface|CreateWidget "/Game/Blueprints/Characters/JetPack/JP_UI/JetpackUI.JetpackUI_C"))
  (bind _output_get (Variables|Default|SetUI _returnvalue))
  (UserInterface|Viewport|AddtoViewport _output_get 0)
  ;[1 1 1] Init author and fuel
  (Variables|Default|SetNewAuthor -2e+02)
  (Variables|Default|SetActualFuel (Variables|/Game/Blueprints/Characters/JetPack/JP_DataAsset/BP_JetPackDataAsset.BP_JetPackDataAsset_C|GetMaxFuel (Variables|Default|GetdataAsset))))

(event Input|KeyboardEvents|LeftShift
  (params (Key :type Key%20Structure :default "None"))
  (bind _ui (Variables|Default|GetUI))
  ;[0 0 0] Up author fly
  (:Pressed
    (Variables|Default|SetUpMaxAuthor? true)
    (if (== (Variables|Default|GetNewAuthor) -2e+02)
      (Variables|Default|SetNewAuthor (+ (Variables|Default|GetNewAuthor) 2e+02))
      ;[1 0.5471 0.09945] spawn jetpack force
      (bind _returnvalue (Game|SpawnActorfromClass "/Game/Blueprints/Characters/JetPack/JP_Projectile/BP_JetpackProjectile.BP_JetpackProjectile_C" (Math|Transform|MakeTransform (Transformation|GetActorLocation (Components|GetOwner))) "Undefined" "OverrideRootScale" 0 0))
      (Variables|/Game/Blueprints/Characters/JetPack/JP_Projectile/BP_JetpackProjectile.BP_JetpackProjectile_C|SetNewAuthor _returnvalue (Variables|Default|GetNewAuthor))
      (Default|ChangeJpForce _ui (Variables|Default|GetNewAuthor) 7e+02 -2e+02) ; Update UI
      ;[0 1 0.8049] Change fuel stock
      (Default|ChangeFuel _ui (Variables|Default|GetActualFuel) (Variables|/Game/Blueprints/Characters/JetPack/JP_DataAsset/BP_JetPackDataAsset.BP_JetPackDataAsset_C|GetMaxFuel (Variables|Default|GetdataAsset))) ; Update UI
    ))
  (:Released
    (Variables|Default|SetUpMaxAuthor? false)))

(event Input|KeyboardEvents|LeftCtrl
  (params (Key :type Key%20Structure :default "None"))
  ;[0 0 0] Reduce author fly
  (:Pressed
    (Variables|Default|SetDownMaxAuthor? true))
  (:Released
    (Variables|Default|SetDownMaxAuthor? false)))

(fn UpMaxAuthor
  (if (< (Variables|Default|GetNewAuthor) 7e+02)
    (Variables|Default|SetNewAuthor (+ (Variables|Default|GetNewAuthor) 1e+01))))

(fn DownMaxAuthor
  (if (> (Variables|Default|GetNewAuthor) -2e+02)
    (Variables|Default|SetNewAuthor (- (Variables|Default|GetNewAuthor) 1e+01))))

(fn Fuel
  (if (< (Variables|Default|GetActualFuel) (Variables|/Game/Blueprints/Characters/JetPack/JP_DataAsset/BP_JetPackDataAsset.BP_JetPackDataAsset_C|GetMaxFuel (Variables|Default|GetdataAsset)))
    (Variables|Default|SetActualFuel (+ (Variables|Default|GetActualFuel) (Variables|/Game/Blueprints/Characters/JetPack/JP_DataAsset/BP_JetPackDataAsset.BP_JetPackDataAsset_C|GetrestorFuel (Variables|Default|GetdataAsset))))))