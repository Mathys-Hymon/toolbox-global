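; A pressure plate gameplay element that reacts when the player character steps on or off its trigger volume.
; Trigger overlaps filtered to BP_ThirdPersonCharacter toggle an IsActive flag and play a sound at the plate's location.
; A PlatePressure timeline plays forward on entry and reverses on exit, lerping the plate mesh's relative Z to sink and raise it.
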(event OnComponentBeginOverlap(Trigger)
  (params (OverlappedComponent :type Primitive%20Component%20Object%20Reference) (OtherActor :type Actor%20Object%20Reference) (OtherComp :type Primitive%20Component%20Object%20Reference) (OtherBodyIndex :type Integer) (bFromSweep :type Boolean) (SweepResult :type Hit%20Result%20Structure%20%28by%20ref%29))
  ;[1 1 1] Player Triggers Pressure Plate
  (Utilities|Casting|CastToBP_ThirdPersonCharacter OtherActor) ; Check overlap with PC
  (Audio|PlaySoundatLocation 0 (Transformation|GetActorLocation) "0, 0, 0" 1.0 1.0 0.0 0 0 0 0) ; ADD SOUND HERE
  (Variables|Default|SetisActive true) ; Sound PLAYING
  (bind _height (Timeline|Plate%20Pressure Play) ; Pressure Animation
    (:Update
      (Transformation|SetRelativeLocation (Variables|Default|GetPressurePlate) (Math|Vector|MakeVector 0.0 0.0 (Math|Float|Lerp 33.0 -2e+01 _height)) false false))))

(event OnComponentEndOverlap(Trigger)
  (params (OverlappedComponent :type Primitive%20Component%20Object%20Reference) (OtherActor :type Actor%20Object%20Reference) (OtherComp :type Primitive%20Component%20Object%20Reference) (OtherBodyIndex :type Integer))
  ;[1 1 1] Player Release Pressure Plate
  (Utilities|Casting|CastToBP_ThirdPersonCharacter OtherActor) ; Check overlap with PC
  (Audio|PlaySoundatLocation 0 (Transformation|GetActorLocation) "0, 0, 0" 1.0 1.0 0.0 0 0 0 0) ; ADD SOUND HERE
  (Variables|Default|SetisActive false) ; Sound STOP
  ;[1 1 1] Player Triggers Pressure Plate
  (bind _height (Timeline|Plate%20Pressure Reverse) ; Pressure Animation
    (:Update
      (Transformation|SetRelativeLocation (Variables|Default|GetPressurePlate) (Math|Vector|MakeVector 0.0 0.0 (Math|Float|Lerp 33.0 -2e+01 _height)) false false))))

(fn ConstructionScript)