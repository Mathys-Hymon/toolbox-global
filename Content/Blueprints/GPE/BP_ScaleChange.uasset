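; BP_ScaleChange is a gameplay element that randomly resizes itself when the player character enters its box trigger.
; On overlap, a random integer picks one of four preset scales for the actor.
; A DoOnce gate fires the change once and resets when the player leaves the box, so each new entry can roll again.
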(event OnComponentBeginOverlap(Box)
  (params (OverlappedComponent :type Primitive%20Component%20Object%20Reference) (OtherActor :type Actor%20Object%20Reference) (OtherComp :type Primitive%20Component%20Object%20Reference) (OtherBodyIndex :type Integer) (bFromSweep :type Boolean) (SweepResult :type Hit%20Result%20Structure%20%28by%20ref%29))
  (if (== OtherActor (Game|GetPlayerCharacter 0))
    (Utilities|FlowControl|DoOnce false
      (:Completed
        (switch int (Math|Random|RandomInteger 4)
          (:0
            (Transformation|SetActorScale3D (Variables|Default|GetScale1)))
          (:1
            (Transformation|SetActorScale3D (Variables|Default|GetScale1_0)))
          (:2
            (Transformation|SetActorScale3D (Variables|Default|GetScale1_1)))
          (:3
            (Transformation|SetActorScale3D (Variables|Default|GetScale1_2))))))))

(event OnComponentEndOverlap(Box)
  (params (OverlappedComponent :type Primitive%20Component%20Object%20Reference) (OtherActor :type Actor%20Object%20Reference) (OtherComp :type Primitive%20Component%20Object%20Reference) (OtherBodyIndex :type Integer))
  (if (== OtherActor (Game|GetPlayerCharacter 0))
    (Utilities|FlowControl|DoOnce false) ; enters at Reset
  ))

(fn ConstructionScript)