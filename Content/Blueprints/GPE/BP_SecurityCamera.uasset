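; Security camera that sweeps between two yaw limits and detects the player with a scalable cone, optionally only while moving.
; Detection line-traces toward the player, stores the hit actor, sets alert material and sound, and turns the camera to track within clamped yaw.
; On overlap end it faces the last seen location, resuming the sweep after a retriggerable delay.
; Construction script previews both sweep limits; BeginPlay removes the preview components.
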(event OnComponentEndOverlap(Cone)
  (params (OverlappedComponent :type Primitive%20Component%20Object%20Reference) (OtherActor :type Actor%20Object%20Reference) (OtherComp :type Primitive%20Component%20Object%20Reference) (OtherBodyIndex :type Integer))
  ;[1 1 1] IfTheCameraDoesn'tDetectThePlayerAnymore
  (Variables|Default|SetlastSeenLoc (Transformation|GetActorLocation OtherActor))
  (Variables|Default|SetseenActorRef 0)
  (Utilities|FlowControl|RetriggerableDelay (Variables|Default|GetdelayWhenLostPlayer))
  (Variables|Default|SetlastSeenLoc "0, 0, 0")
  (Variables|Default|SetseePlayer false)
  (Rendering|Material|SetMaterial (Variables|Default|GetCone) 0 (Variables|Default|GetcamDefaultMat)))

(event EventBeginPlay
  (bind _detectionsize (Variables|Default|GetdetectionSize))
  ;[1 0.3306 0] BeginPlay
  (Transformation|SetWorldScale3D (Variables|Default|GetCone) (Math|Vector|MakeVector _detectionsize _detectionsize (Variables|Default|GetdetectionLength)))
  (Transformation|SetRelativeRotation (Variables|Default|GetCamera) (Math|Rotator|MakeRotator 0.0 (Variables|Default|GetdetectionAngle) 0.0) false false)
  (for _array_element (Utilities|Array|MakeArray (Variables|Default|GetCameraPreview1) (Variables|Default|GetCone1) (Variables|Default|GetCone2) (Variables|Default|GetCameraPreview2))
    (Components|DestroyComponent _array_element)))

(event EventTick
  (params (DeltaSeconds :type Float%20%28single-precision%29))
  (bind _cone (Variables|Default|GetCone))
  (bind _camera (Variables|Default|GetCamera))
  (bind _camera_2 (Variables|Default|GetCamera))
  (bind _playerclass (Variables|Default|GetplayerClass))
  (bind _overlappingactors (Collision|GetOverlappingActors _cone _playerclass :!class /Script/Engine.PrimitiveComponent))
  (bind _relativerotation (Variables|/Script/Engine.SceneComponent|GetRelativeRotation _camera))
  (bind _relativerotation_2 (Variables|/Script/Engine.SceneComponent|GetRelativeRotation _camera_2))
  (bind _output (Utilities|Array|Get(acopy) _overlappingactors))
  ;[0.2717 1 0] Tick
  (Utilities|FlowControl|Sequence
    (:then_0
      ;[1 1 1] Rotation
      (if (not (Variables|Default|GetseePlayer))
        (if (Math|Float|NearlyEqual(Float) (.yaw _relativerotation) (Variables|Default|GetmaxRotationAngle) 0.5)
          (Variables|Default|SetgoRight true)
          (elif (Math|Float|NearlyEqual(Float) (.yaw _relativerotation) (Variables|Default|GetminRotationAngle) 0.5)
            (Variables|Default|SetgoRight false)))
        (Transformation|SetRelativeRotation _camera_2 (Math|Rotator|MakeRotator (.roll _relativerotation_2) (.pitch _relativerotation_2) (Math|Interpolation|FInterptoConstant (.yaw _relativerotation_2) (Math|Float|SelectFloat (Variables|Default|GetminRotationAngle) (Variables|Default|GetmaxRotationAngle) (Variables|Default|GetgoRight)) (Utilities|Time|GetWorldDeltaSeconds) (Variables|Default|GetInterp%20Speed))) false false)))
    (:then_1
      ;[1 1 1] RotateCameraTowardPlayer
      (if (Variables|Default|GetseePlayer)
        (Utilities|IsValid (Variables|Default|GetseenActorRef)
          (:Is%20Valid
            (CallFunction|RotatewhenSeen (Transformation|GetActorLocation (Variables|Default|GetseenActorRef))))
          (:Is%20Not%20Valid
            (CallFunction|RotatewhenSeen (Variables|Default|GetlastSeenLoc))))))
    (:then_2
      ;[1 1 1] DetectIfPlayerIsMovingInTheDetectionRange
      (Utilities|IsValid _output
        (:Is%20Valid
          (if (Variables|Default|GetisMotionTriggered)
            (if (> (Math|Vector|VectorLength (Transformation|GetVelocity _output)) 0.0)
              (bind _outhit (Collision|LineTraceByChannel (Transformation|GetWorldLocation (Variables|Default|GetCamera)) (Transformation|GetActorLocation _output) "TraceTypeQuery1" false 0 "None" :!label _label))
              (Variables|Default|SetseenActorRef (.HitActor (Collision|BreakHitResult _outhit)))
              (Variables|Default|SetseePlayer true)
              (Rendering|Material|SetMaterial (Variables|Default|GetCone) 0 (Variables|Default|GetcamAlertMat))
              (Audio|PlaySound2D (Variables|Default|GetcamAlertSound) 0.4 1.0 0.0 0 0))
            (else
              (goto _label))))))))

(fn ConstructionScript
  (bind _detectionsize (Variables|Default|GetdetectionSize))
  (bind _detectionsize_2 (Variables|Default|GetdetectionSize))
  (bind _detectionsize_3 (Variables|Default|GetdetectionSize))
  (Utilities|FlowControl|Sequence
    (:then_0
      (Transformation|SetWorldScale3D (Variables|Default|GetCone) (Math|Vector|MakeVector _detectionsize_3 _detectionsize_3 (Variables|Default|GetdetectionLength)))
      (Transformation|SetRelativeRotation (Variables|Default|GetCamera) (Math|Rotator|MakeRotator 0.0 (Variables|Default|GetdetectionAngle) 0.0) false false))
    (:then_1
      (Transformation|SetWorldScale3D (Variables|Default|GetCone1) (Math|Vector|MakeVector _detectionsize_2 _detectionsize_2 (Variables|Default|GetdetectionLength)))
      (Transformation|SetRelativeRotation (Variables|Default|GetCameraPreview1) (Math|Rotator|MakeRotator 0.0 (Variables|Default|GetdetectionAngle) (Variables|Default|GetminRotationAngle)) false false))
    (:then_2
      (Transformation|SetWorldScale3D (Variables|Default|GetCone2) (Math|Vector|MakeVector _detectionsize _detectionsize (Variables|Default|GetdetectionLength)))
      (Transformation|SetRelativeRotation (Variables|Default|GetCameraPreview2) (Math|Rotator|MakeRotator 0.0 (Variables|Default|GetdetectionAngle) (Variables|Default|GetmaxRotationAngle)) false false))))

(fn RotatewhenSeen
  (params (Start :type Vector%20%28by%20ref%29))
  (bind _camera (Variables|Default|GetCamera))
  (bind _relativerotation (Variables|/Script/Engine.SceneComponent|GetRelativeRotation _camera))
  (Transformation|SetRelativeRotation _camera (Math|Rotator|MakeRotator (.roll _relativerotation) (.pitch _relativerotation) (Math|Float|Clamp(Float) (Math|Interpolation|FInterptoConstant (.yaw _relativerotation) (.yaw (Math|Rotator|FindLookatRotation Start (Transformation|GetWorldLocation (Variables|Default|GetCamera)))) (Utilities|Time|GetWorldDeltaSeconds) 3e+01) -45.0 45.0)) false false)
  (return))