(fn Dialogue
  ;[1 1 1] Tutorial Dialgoue Tree
  (Development|PrintString "Conversation Started")
  (|CallParentFunction)
  (switch int (Variables|Default|GetDialogueTreeIndex) ; Branching Dialogue\n(Starts at 0)
    (:0
      (Development|PrintString "Index 0.0")
      (bind _optionindex (CallFunction|AddDialogue "Tutorial" "Hello! Welcome to Karris' dialogue Tutorial. What do you want to know first?" (Utilities|Array|MakeArray "How to Add Dialogue?" "How to Add Options to Dialogue?"))) ; Add Your Dialogue
      (Development|PrintString "Add Dialogue")
      (switch Utilities|FlowControl|Switch|SwitchonENUM_DialogueState "NewEnumerator0"
        (:NewEnumerator0
          (switch int _optionindex ; Pins here directly correlate to\nthe index of the Options 0=0 1=1
            (:0
              (Development|PrintString "Index 1.0")
              (bind (_state _optionindex_2) (CallFunction|AddDialogue "Tutorial" "Add Dialogue? First take a look at the \"AC_Dialogue_Tutorial\" to see how branching Dialogue is created. You can \"Add Dialogue\" which is a function. Then make a switch branching into the options and response, depending on your choices." (Utilities|Array|MakeArray "I'd like to ask another question." "I'm finished with my questons."))) ; Option 1 - Pin 1
              (switch Utilities|FlowControl|Switch|SwitchonENUM_DialogueState _state
                (:NewEnumerator0
                  (switch int _optionindex_2 ; Pins here directly correlate to\nthe index of the Options 0=0 1=1
                    (:0
                      (CallFunction|SetDialogueTreeIndex) ; Return to Exact Index
                      (Development|PrintString "Return to Index 0.0"))
                    (:1
                      (CallFunction|SetDialogueTreeIndex 1) ; Return to Exact Index
                      (CallFunction|CloseConversation) ; End Dialogue
                      (Development|PrintString "End Conversation"))))))
            (:1
              (Development|PrintString "Index 1.2")
              (bind (_state_2 _optionindex_3) (CallFunction|AddDialogue "Tutorial" "To add Options to a Dialogue box, check \"AC_Dialogue_Tutorial\", you'll see after adding Dialogue you make an Array of Options, then directly add pins to type out your different Dialogue Options!" (Utilities|Array|MakeArray "I'd like to ask another question." "I'm finished with my questions."))) ; Add Your Dialogue
              (switch Utilities|FlowControl|Switch|SwitchonENUM_DialogueState _state_2
                (:NewEnumerator0
                  (switch int _optionindex_3 ; Pins here directly correlate to\nthe index of the Options 0=0 1=1
                    (:0
                      (CallFunction|SetDialogueTreeIndex) ; Return to Exact Index
                    )
                    (:1
                      (CallFunction|SetDialogueTreeIndex 1) ; Return to Exact Index
                      (CallFunction|CloseConversation) ; End Dialogue
                      (Development|PrintString "Index 1.1"))))))
            (:2
              (Development|PrintString "Index 1.3")
              (bind (_state_3 _optionindex_4) (CallFunction|AddDialogue "Tutorial" "To add Options to a Dialogue box, check \"AC_Dialogue_Tutorial\", you'll see after adding Dialogue you make an Array of Options, then directly add pins to type out your different Dialogue Options!")) ; Add Your Dialogue
              (switch Utilities|FlowControl|Switch|SwitchonENUM_DialogueState _state_3
                (:NewEnumerator0
                  (switch int _optionindex_4 ; Pins here directly correlate to\nthe index of the Options 0=0 1=1
                    (:0
                      (CallFunction|SetDialogueTreeIndex) ; Return to Exact Index
                    )
                    (:1
                      (CallFunction|SetDialogueTreeIndex 1) ; Return to Exact Index
                      (CallFunction|CloseConversation) ; End Dialogue
                      (Development|PrintString "Index 1.1"))))))))))
    (:1
      (Development|PrintString "Index 0.1")
      ;;[1 1 1] Finish Tutorial : Randomized Thank You
      (bind _optionindex_5 (CallFunction|AddDialogue "" (Utilities|Select :Index (Math|Random|RandomIntegerinRange 0 1) :Option%200 "Thank you for using my Dialogue Tool!" :Option%201 "Hope you enjoy using my Dialogue Tool!") (Utilities|Array|MakeArray "End Conversation")))
      (switch Utilities|FlowControl|Switch|SwitchonENUM_DialogueState "NewEnumerator0"
        (:NewEnumerator0
          (switch int _optionindex_5 ; Pins here directly correlate to\nthe index of the Options 0=0 1=1
            (:0
              (CallFunction|ClearDialogueProgress)
              (CallFunction|CloseConversation) ; End Dialogue
            )))))))