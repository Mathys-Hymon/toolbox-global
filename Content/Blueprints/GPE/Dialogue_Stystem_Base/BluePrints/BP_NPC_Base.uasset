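; Base NPC actor for the dialogue system, with a character name label and hooks for interaction.
; The construction script fills the label from CharacterName, and SetInteractableState shows or hides it according to whether interaction is available.
; When a conversation closes, it notifies the interaction instigator through ConversationClosedMessage so movement can be re-enabled.
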(event EventConversationClosed
  ;[1 1 1] End Conversation - Reenable Movement
  (Class|BPIInteractable|ConversationClosed(Message) (Variables|Default|GetInteractInstagator)))

(event EventSetInteractableState
  (params (CanShowIneteract? :type Boolean))
  ;[1 1 1] PopUp Visibility
  (if CanShowIneteract?
    (Rendering|SetVisibility (Variables|Default|GetTXT_CharacterName) true false)
    (else
      (Rendering|SetVisibility (Variables|Default|GetTXT_CharacterName) false false) ; Invisible Until Set Range
    )))

(fn ConstructionScript
  ;[1 1 1] Add NPC Name
  (Rendering|Components|TextRender|SetText (Variables|Default|GetTXT_CharacterName) (Variables|Default|GetCharacterName)))