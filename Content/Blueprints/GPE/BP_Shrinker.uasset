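; BP_Shrinker is a gameplay element whose sphere shrinks or grows when an actor enters its detection radius, depending on ShrinkOrGrow.
; Begin overlap resets the actor to BigSize, then plays a timeline, rate-scaled by duration, that lerps the sphere's world scale.
; End overlap reverses the timeline, after RefreshDelay when growing; actors tagged "Shrinker" are ignored.
; The construction script sizes the trigger collider from DetectionRadius.
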(event OnComponentBeginOverlap(Collider)
  (params (OverlappedComponent :type Primitive%20Component%20Object%20Reference) (OtherActor :type Actor%20Object%20Reference) (OtherComp :type Primitive%20Component%20Object%20Reference) (OtherBodyIndex :type Integer) (bFromSweep :type Boolean) (SweepResult :type Hit%20Result%20Structure%20%28by%20ref%29))
  ;[0.04167 0.04167 0.04167] Shrink/Grow
  ;;[0.04167 0.04167 0.04167] Shrink
  (if (Variables|Default|GetShrinkOrGrow) ; If Shrinker or Grower
    (if (not (Actor|ActorHasTag OtherActor "Shrinker"))
      (Transformation|SetActorRelativeScale3D (Variables|Default|GetBigSize))
      (Components|Timeline|SetPlayRate (Variables|Default|GetShrink) (/ 1.0 (Variables|Default|GetDurationShrink)))
      (bind _size (Timeline|Shrink Play) ; Shrinking animation
        (:Update
          (Transformation|SetWorldScale3D (Variables|Default|GetSphere) (Math|Vector|Lerp(Vector) (Variables|Default|GetBigSize) (Variables|Default|GetSmallSize) _size)))))
    (elif (not (Actor|ActorHasTag OtherActor "Shrinker"))
      (Transformation|SetActorRelativeScale3D (Variables|Default|GetBigSize))
      (Components|Timeline|SetPlayRate (Variables|Default|GetGrow) (/ 1.0 (Variables|Default|GetDurationGrow)))
      (bind _grow (Timeline|Grow Play) ; Growing animation
        (:Update
          (Transformation|SetWorldScale3D (Variables|Default|GetSphere) (Math|Vector|Lerp(Vector) (Variables|Default|GetBigSize) (Variables|Default|GetBiggerSize) _grow)))))))

(event OnComponentEndOverlap(Collider)
  (params (OverlappedComponent :type Primitive%20Component%20Object%20Reference) (OtherActor :type Actor%20Object%20Reference) (OtherComp :type Primitive%20Component%20Object%20Reference) (OtherBodyIndex :type Integer))
  ;[0.04167 0.04167 0.04167] Shrink/Grow
  ;;[0.03646 0.03646 0.03646] Grow
  (if (Variables|Default|GetShrinkOrGrow)
    (if (not (Actor|ActorHasTag OtherActor "Shrinker"))
      (bind _size (Timeline|Shrink Reverse) ; Shrinking animation
        (:Update
          (Transformation|SetWorldScale3D (Variables|Default|GetSphere) (Math|Vector|Lerp(Vector) (Variables|Default|GetBigSize) (Variables|Default|GetSmallSize) _size)))))
    (elif (not (Actor|ActorHasTag OtherActor "Shrinker"))
      (Utilities|FlowControl|Delay (Variables|Default|GetRefreshDelay))
      (bind _grow (Timeline|Grow Reverse) ; Growing animation
        (:Update
          (Transformation|SetWorldScale3D (Variables|Default|GetSphere) (Math|Vector|Lerp(Vector) (Variables|Default|GetBigSize) (Variables|Default|GetBiggerSize) _grow)))))))

(fn ConstructionScript
  (Components|Sphere|SetSphereRadius (Variables|Default|GetCollider) (Variables|Default|GetDetection%20Radius) true))