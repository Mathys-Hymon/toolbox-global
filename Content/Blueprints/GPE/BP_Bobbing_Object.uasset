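; BP_Bobbing_Object is an actor that spins and bobs up and down continuously, likely as a gameplay element.
; BeginPlay stores the Cube component's relative Z as the base height.
; Each Tick adds yaw rotation scaled by delta time, then offsets the Cube's relative Z with a degree-based sine of time since creation, using tunable speed and distance.
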(event EventTick
  (params (DeltaSeconds :type Float%20%28single-precision%29))
  ;[1 1 1] Rotate Object
  (Transformation|AddActorLocalRotation (Math|Rotator|MakeRotator 0.0 0.0 (* DeltaSeconds (Variables|Default|GetYaw%20Persecond))) false false) ; Add rotation to object
  (Transformation|SetRelativeLocation (Variables|Default|GetCube) (Math|Vector|MakeVector 0.0 0.0 (+ (Variables|Default|GetRelative%20Starting%20Location%20Z) (* (Math|Trig|Sin(Degrees) (* (Actor|GetGameTimeSinceCreation) (Variables|Default|GetBobbing%20Speed))) (Variables|Default|GetBobbing%20Distance)))) false false) ; Add bobbing
)

(event EventBeginPlay
  ;[1 1 1] Begin Play
  (Variables|Default|SetRelative%20Starting%20Location%20Z (.z (.location (Transformation|GetRelativeTransform (Variables|Default|GetCube))))) ; Set as Starting Z axis
)

(fn ConstructionScript)