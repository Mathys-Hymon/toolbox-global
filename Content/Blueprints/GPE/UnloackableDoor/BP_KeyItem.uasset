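; BP_KeyItem is a pickup actor that adds its KeyItem to the player's inventory, then destroys itself.
; A detection box, scaled in the construction script, either triggers immediate collection on player overlap when AutoPickUp is set, or flags the player as in range.
; In manual mode, Tick polls the player's HasInteracted flag while in range to collect the item.
; It depends on BP_CharacterWithAdaptativeCameraV1 for input and inventory.
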(event OnComponentBeginOverlap(DetectionBox)
  (params (OverlappedComponent :type Primitive%20Component%20Object%20Reference) (OtherActor :type Actor%20Object%20Reference) (OtherComp :type Primitive%20Component%20Object%20Reference) (OtherBodyIndex :type Integer) (bFromSweep :type Boolean) (SweepResult :type Hit%20Result%20Structure%20%28by%20ref%29))
  ;[0.1255 0.5216 0.5255] Add the itemStructure to the player inventory and delete the actor
  (if (== OtherActor (Variables|Default|GetPlayer%20Character)) ; Check if overlap is trigger by player
    (if (Variables|KeySettings|GetautoPickUp) ; Check if this item is auto picked or not
      (Default|AddtoInventory (Variables|Default|GetPlayer%20Character) (Variables|Default|GetKeyItem)) ; You can change for your inventory system
      (Development|PrintString "Item picked up")
      (Actor|DestroyActor)
      (else
        (Variables|KeySettings|SetisInRange true)))
    (else
      (Development|PrintString "This character is not the player"))))

(event OnComponentEndOverlap(DetectionBox)
  (params (OverlappedComponent :type Primitive%20Component%20Object%20Reference) (OtherActor :type Actor%20Object%20Reference) (OtherComp :type Primitive%20Component%20Object%20Reference) (OtherBodyIndex :type Integer))
  ;[0.1255 0.5216 0.5255] Check if player is still in range
  (if (== OtherActor (Variables|Default|GetPlayer%20Character))
    (Variables|KeySettings|SetisInRange false)))

(event EventBeginPlay
  (bind _asbp_character_with_adaptative_camera_v1 (Utilities|Casting|CastToBP_CharacterWithAdaptativeCameraV1 (Game|GetPlayerCharacter 0)))
  (Variables|Default|SetPlayer%20Character _asbp_character_with_adaptative_camera_v1))

(event EventTick
  (params (DeltaSeconds :type Float%20%28single-precision%29))
  (bind _player_character (Variables|Default|GetPlayer%20Character))
  ;[0.1255 0.5216 0.5255] This will only be executed if the autoPickUp is disable as the item will wait for an input (Has Interacted) before being collected
  (if (and (Variables|/Game/Blueprints/Characters/BP_CharacterWithAdaptativeCameraV1.BP_CharacterWithAdaptativeCameraV1_C|GethasInteracted _player_character) (Variables|KeySettings|GetisInRange))
    (Default|AddtoInventory _player_character (Variables|Default|GetKeyItem))
    (Development|PrintString "Item picked up")
    (Actor|DestroyActor)))

(fn ConstructionScript
  ;[0 1 0] Set the detection box size
  (Transformation|SetWorldScale3D (Variables|Default|GetDetection%20Box) (Variables|KeySettings|GetdetectionBoxSize))
  ;[0 1 0] Set the static mesh as the static mesh assigned in the itemStructure
  (Components|StaticMesh|SetStaticMesh (Variables|Default|GetKey%20Mesh) 0))