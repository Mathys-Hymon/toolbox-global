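; BP_Objective is an objective marker actor that tracks its distance to the player character.
; On BeginPlay it caches a BP_FirstPersonCharacter reference and adds a WB_HUDMarker widget to the viewport.
; Each Tick it passes the distance to that character to the WB_Marker in its widget component and stores it in DistanceToObject.
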(event EventBeginPlay
  ;[1 1 1] Get player character reference
  (bind _asbp_first_person_character (Utilities|Casting|CastToBP_FirstPersonCharacterClass "/Game/FirstPerson/Blueprints/BP_FirstPersonCharacter.BP_FirstPersonCharacter_C"))
  (bind _returnvalue (Actor|GetActorOfClass _asbp_first_person_character))
  (Variables|Default|SetCharacterRef _returnvalue)
  (bind _returnvalue_2 (UserInterface|CreateWidget "/Game/Blueprints/Marker/WB_HUDMarker.WB_HUDMarker_C"))
  (UserInterface|Viewport|AddtoViewport _returnvalue_2 0))

(event EventTick
  (params (DeltaSeconds :type Float%20%28single-precision%29))
  (bind _characterref (Variables|Default|GetCharacterRef))
  (bind _returnvalue (Transformation|GetDistanceTo _characterref))
  (bind _asw_marker (Utilities|Casting|CastToWB_Marker (UserInterface|GetWidget (Variables|Default|GetWidget))))
  (Default|EventUpdateDistance _asw_marker _returnvalue)
  (Variables|Default|SetDistanceToObject _returnvalue))

(fn ConstructionScript)