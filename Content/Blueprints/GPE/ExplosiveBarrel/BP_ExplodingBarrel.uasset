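; Explosive barrel that burns when damaged and explodes when its life runs out, pushing and damaging nearby actors.
; Non-lethal damage or a debug box overlap starts burning, which swaps the material and drains life on a looping timer.
; Lethal damage triggers a randomly delayed sphere trace that sends impulse and damage messages through BPI_ExplodingBarrel, then destroys the barrel.
; The barrel's own Explodes event applies a radial impulse to its mesh.
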(event OnComponentBeginOverlap(Box)
  (params (OverlappedComponent :type Primitive%20Component%20Object%20Reference) (OtherActor :type Actor%20Object%20Reference) (OtherComp :type Primitive%20Component%20Object%20Reference) (OtherBodyIndex :type Integer) (bFromSweep :type Boolean) (SweepResult :type Hit%20Result%20Structure%20%28by%20ref%29))
  ;[1 1 1] Debug Stuff (you can delete this)
  (Utilities|Casting|CastTo OtherActor)
  (CallFunction|Burn))

(event Custom|Burn
  ;[1 1 1] If the damages are not enough to destroy the barrel, the barel will burn
  (Rendering|Material|SetMaterial (Variables|Default|GetBarrelMesh) 0 "/Game/Blueprints/GPE/ExplosiveBarrel/M_IsExplodingPlaceHolder.M_IsExplodingPlaceHolder")
  (Utilities|Time|SetTimerbyEvent (delegate Custom|Burn) 0.5 true true)
  (bind _output_get (Variables|Default|Setlife (- (Variables|Default|Getlife) 1.0)))
  (if (<= _output_get 0.0)
    (CallFunction|TakeDamages 1.0)))

(event EventTakeDamages
  (params (damages :type Float%20%28double-precision%29))
  (bind _barrelmesh (Variables|Default|GetBarrelMesh))
  (bind _returnvalue (Transformation|GetWorldLocation _barrelmesh))
  ;[1 1 1] If The life is < 0, the barrel Explodes
  (if (<= (- (Variables|Default|Getlife) damages) 0.0)
    (Utilities|FlowControl|Delay (Math|Random|RandomFloatinRange (Variables|Default|GetminTimeBeforeExplosion) (Variables|Default|GetmaxTimeBeforeExplosion)))
    (bind _outhits (Collision|MultiSphereTraceByChannel _returnvalue _returnvalue (Variables|Default|GetexplosionRadius) "TraceTypeQuery1" false 0 "ForDuration"))
    (for _array_element _outhits
      (if (Utilities|DoesObjectImplementInterface (.HitActor (Collision|BreakHitResult _array_element)) "/Game/Blueprints/GPE/ExplosiveBarrel/BPI_ExplodingBarrel.BPI_ExplodingBarrel_C")
        (Class|BPIExplodingBarrel|Explodes(Message) (.HitActor (Collision|BreakHitResult _array_element)) (Transformation|GetWorldLocation (Variables|Default|GetBarrelMesh)) (Variables|Default|GetexplosionForce) (Variables|Default|GetexplosionRadius))
        (Class|BPIExplodingBarrel|TakeDamages(Message) (.HitActor (Collision|BreakHitResult _array_element)) (Variables|Default|Getdamages)))
      (Utilities|FlowControl|DelayUntilNextTick)
      (Actor|DestroyActor))
    (else
      (CallFunction|Burn))))

(event EventExplodes
  (params (originExplosion :type Vector :default "0, 0, 0") (explosionForce :type Float%20%28double-precision%29) (radiusExplosion :type Float%20%28double-precision%29))
  ;[0.1888 1 0] You can add this event to every objects you want to react the explosion (just add the BPI in the object)
  (Physics|AddRadialImpulse (Variables|Default|GetBarrelMesh) originExplosion radiusExplosion explosionForce "RIF_Constant" true))

(fn ConstructionScript)