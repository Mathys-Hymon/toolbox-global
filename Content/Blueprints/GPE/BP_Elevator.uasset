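; BP_Elevator is an elevator that travels between a start and an end position when the player pawn enters its Box trigger.
; On BeginPlay it sets the timeline play rate and computes the end position from an offset multiplied by the root's world scale.
; Each overlap while idle plays or reverses the timeline, which lerps the actor's location.
; On finish, the timeline direction updates which end the elevator rests at.
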(event OnComponentBeginOverlap(Box)
  (params (OverlappedComponent :type Primitive%20Component%20Object%20Reference) (OtherActor :type Actor%20Object%20Reference) (OtherComp :type Primitive%20Component%20Object%20Reference) (OtherBodyIndex :type Integer) (bFromSweep :type Boolean) (SweepResult :type Hit%20Result%20Structure%20%28by%20ref%29))
  ;[1 1 1] Checks if Elevator should Elevate
  (if (== OtherActor (Game|Player|GetPlayerPawn 0))
    (if (not (Variables|Default|GetIsMoving?))
      (Variables|Default|SetIsMoving? true)
      ;[1 1 1] Move Elevator to Start or End depending on which it is now
      (if (Variables|Default|GetAtStart?)
        (bind (_direction _newtrack_0) (Timeline|MoveElevatorTimeline PlayFromStart)
          (:Update
            (Transformation|SetActorLocation (Math|Vector|Lerp(Vector) (Variables|Default|GetStartPos) (Variables|Default|GetEndPosition) _newtrack_0) false false))
          (:Finished
            (Variables|Default|SetIsMoving? false)
            (Variables|Default|SetAtStart? (Utilities|Select :Index _direction :Forward false :Backward true))))
        (else
          (Timeline|MoveElevatorTimeline Reverse))))))

(event EventBeginPlay
  (bind _endpossetup (Variables|Default|GetEndPosSetup))
  (bind _defaultsceneroot (Variables|Default|GetDefaultSceneRoot))
  (bind _returnvalue (Transformation|GetWorldScale _defaultsceneroot))
  ;[1 1 1] Sets up End and Start Position as well as Playrate of the timeline
  (Components|Timeline|SetPlayRate (Variables|Default|GetMoveElevatorTimeline) (Variables|Default|GetPlayrate))
  ;;[1 1 1] Setup for End position, If not done like this, doesn't take into account the scale and might go not far enough or too far
  (Variables|Default|SetEndPosition (+ (Variables|/Script/Engine.SceneComponent|GetRelativeLocation _defaultsceneroot) (Math|Vector|MakeVector (* (.x _endpossetup) (.x _returnvalue)) (* (.y _endpossetup) (.y _returnvalue)) (* (.z _endpossetup) (.z _returnvalue)))))
  (Variables|Default|SetStartPos (Transformation|GetWorldLocation (Variables|Default|GetDefaultSceneRoot))))

(event EventTick
  (params (DeltaSeconds :type Float%20%28single-precision%29)))

(fn ConstructionScript)