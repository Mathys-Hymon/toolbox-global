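; An on-rails camera actor whose camera slides along a spline path to follow the player.
; While the camera is active, Tick smoothly interpolates it toward a target point on the spline.
; The target's spline distance scales with the player's distance from PointA relative to the PointA-to-PointB span.
; When the player is farther than that span from either point, the target holds at the last computed spline position.
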(event EventBeginPlay
  (|CallParentFunction) ; This node is disabled and will not be called.\nDrag off pins to build functionality.
)

(event EventTick
  (params (DeltaSeconds :type Float%20%28single-precision%29))
  (bind _camera (Variables|Default|GetCamera))
  (|CallParentFunction DeltaSeconds)
  (if (Variables|Default|GetActiveCamera)
    (bind _targetcamposition (CallFunction|GetCamPositionRelativetoPlayer (Transformation|GetActorLocation (Game|Player|GetPlayerPawn 0))))
    (Transformation|SetWorldLocation _camera (Math|Interpolation|VInterpTo (Transformation|GetWorldLocation _camera) _targetcamposition (Utilities|Time|GetWorldDeltaSeconds) (Variables|Modifiers|GetInterp%20Speed)) false false)))

(fn ConstructionScript
  (|CallParentFunction))

(fn GetCamPositionRelativetoPlayer
  (params (PlayerPosition :type Vector))
  (bind _path (Variables|Default|GetPath))
  (Variables|Logic|SetDistanceOfTrackPoints (Math|Vector|Distance(Vector) (Transformation|GetWorldLocation (Variables|Default|GetPointA)) (Transformation|GetWorldLocation (Variables|Default|GetPointB))))
  (if (and (<= (Math|Vector|Distance(Vector) (Transformation|GetWorldLocation (Variables|Default|GetPointA)) PlayerPosition) (Variables|Logic|GetDistanceOfTrackPoints)) (<= (Math|Vector|Distance(Vector) (Transformation|GetWorldLocation (Variables|Default|GetPointB)) PlayerPosition) (Variables|Logic|GetDistanceOfTrackPoints)))
    (bind _output_get (Variables|Logic|SetLastCamPosition (* (Spline|GetSplineLength _path) (/ (Math|Vector|Distance(Vector) (Transformation|GetWorldLocation (Variables|Default|GetPointA)) PlayerPosition) (Variables|Logic|GetDistanceOfTrackPoints)))))
    (return (Spline|GetLocationatDistanceAlongSpline _path _output_get "World"))
    (else
      (return (Spline|GetLocationatDistanceAlongSpline (Variables|Default|GetPath) (Variables|Logic|GetLastCamPosition) "World")))))