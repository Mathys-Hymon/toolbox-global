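; Fixed camera actor that becomes the player's view when the player enters either of its two trigger volumes.
; An interface check filters overlaps, then the view blends over BlendTime and the player character receives the camera reference.
; A DefaultCamera flag makes it the starting view on BeginPlay.
; View-target events track whether it is active, and Tick aims the active camera at the player when FocusOnPlayer is set.
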(event OnComponentBeginOverlap(StartTriggerA)
  (params (OverlappedComponent :type Primitive%20Component%20Object%20Reference) (OtherActor :type Actor%20Object%20Reference) (OtherComp :type Primitive%20Component%20Object%20Reference) (OtherBodyIndex :type Integer) (bFromSweep :type Boolean) (SweepResult :type Hit%20Result%20Structure%20%28by%20ref%29))
  ;[1 1 1] Set as Active Camera when Trigger is entered by Player
  (bind _yes (Class|BPIPlayer|IsPlayer(Message) OtherActor)) ; Check Read Me to make sure this is set on your player correctly
  (if _yes
    (Game|Player|SetViewTargetwithBlend (Game|GetPlayerController 0) self (Variables|Behaviour|GetBlend%20Time) "VTBlend_Linear" 0.0 false)
    (Class|BPIPlayer|UpdateCameraComponent(Message) (Game|GetPlayerCharacter 0) (Variables|Default|GetCamera))))

(event OnComponentBeginOverlap(StartTriggerB)
  (params (OverlappedComponent :type Primitive%20Component%20Object%20Reference) (OtherActor :type Actor%20Object%20Reference) (OtherComp :type Primitive%20Component%20Object%20Reference) (OtherBodyIndex :type Integer) (bFromSweep :type Boolean) (SweepResult :type Hit%20Result%20Structure%20%28by%20ref%29))
  ;[1 1 1] Set as Active Camera when Trigger is entered by Player
  (bind _yes (Class|BPIPlayer|IsPlayer(Message) (stale OnComponentBeginOverlap(StartTriggerA) OtherActor))) ; Check Read Me to make sure this is set on your player correctly
  (if _yes
    (Game|Player|SetViewTargetwithBlend (Game|GetPlayerController 0) self (Variables|Behaviour|GetBlend%20Time) "VTBlend_Linear" 0.0 false)
    (Class|BPIPlayer|UpdateCameraComponent(Message) (Game|GetPlayerCharacter 0) (Variables|Default|GetCamera))))

(event EventBeginPlay
  ;[1 1 1] First Camera Setup
  (if (Variables|Behaviour|GetDefaultCamera)
    (Game|Player|SetViewTargetwithBlend (Game|GetPlayerController 0) self 0.0 "VTBlend_Linear" 0.0 false)
    ;[1 1 1] Set as Active Camera when Trigger is entered by Player
    (Class|BPIPlayer|UpdateCameraComponent(Message) (Game|GetPlayerCharacter 0) (Variables|Default|GetCamera))))

(event EventTick
  (params (DeltaSeconds :type Float%20%28single-precision%29))
  (bind _camera (Variables|Default|GetCamera))
  (if (and (Variables|State|GetActiveCamera) (Variables|Behaviour|GetFocusOnPlayer))
    (Transformation|SetWorldRotation _camera (Math|Interpolation|RInterpTo (Transformation|GetWorldRotation _camera) (Math|Rotator|FindLookatRotation (Transformation|GetWorldLocation (Variables|Default|GetCamera)) (Transformation|GetActorLocation (Game|GetPlayerCharacter 0))) (Utilities|Time|GetWorldDeltaSeconds) 0.0) false false)))

(event EventUpdateCamera)

(event EventOnBecomeViewTarget
  (params (PC :type Player%20Controller%20Object%20Reference))
  ;[1 1 1] Current Camera Checks
  (Variables|State|SetActiveCamera true))

(event EventOnEndViewTarget
  (params (PC :type Player%20Controller%20Object%20Reference))
  ;[1 1 1] Current Camera Checks
  (Variables|State|SetActiveCamera false))

(fn ConstructionScript)

(fn GetCamera
  (return (Variables|Default|GetCamera)))