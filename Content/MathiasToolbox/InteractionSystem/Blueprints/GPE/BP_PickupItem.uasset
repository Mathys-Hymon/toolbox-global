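; BP_PickupItem is a pickup GPE for the interaction system that disappears when an actor interacts with it.
; Interact prints a message saying the item was added to the interactor's inventory, plays a click sound at its location and destroys the actor; no inventory data is actually stored.
; SetAnimation supplies the InteractAnimation variable, while SetUI returns a zero draw size and location.
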(event EventInteract
  (params (Interactor :type Actor%20Object%20Reference))
  (Development|PrintString (Utilities|String|ToString(Text) (Utilities|Text|FormatText "Added {ItemName} to the Inventory of {ActorName}" (Utilities|GetDisplayName self) (Utilities|GetDisplayName Interactor))))
  (Audio|PlaySoundatLocation "/Engine/VREditor/Sounds/VR_click3.VR_click3" (Transformation|GetActorLocation) "0, 0, 0" 1.0 1.0 0.0 0 0 0 0)
  (Actor|DestroyActor))

(fn ConstructionScript)

(fn SetAnimation
  (return (Variables|Default|GetInteractAnimation)))

(fn SetUI
  (return "" "0, 0, 0"))